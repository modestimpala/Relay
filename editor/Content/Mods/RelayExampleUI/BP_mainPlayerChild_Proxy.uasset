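; BP_mainPlayerChild_Proxy is a main-player child that acts as a Relay networked proxy pawn with voice chat.
; On BeginPlay it deactivates mic, movement and camera, and snaps the weapon to the Relay held-item anchor.
; After a short delay it binds a voice sink for its authority peer to VoiceChat and opens the preferred voice device.
; Each tick it moves the Relay camera anchor to the networked camera transform when valid.
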(event EventBeginPlay
  (bind _self self)
  (|CallParentFunction)
  (Components|Activation|Deactivate (Variables|Default|Getmic))
  (Components|Activation|Deactivate (Variables|Character|GetCharacterMovement))
  (Components|Activation|Deactivate (Variables|Default|GetCamera))
  (Variables|/Script/Engine.SpringArmComponent|SetbUsePawnControlRotation (Variables|Default|Getlag) false)
  (Transformation|AttachComponentToComponent (Variables|Default|Getweapon) (Variables|Default|GetRelayHeldItemAnchor) "None" "SnapToTarget" "SnapToTarget" "KeepRelative" false)
  (Utilities|FlowControl|Delay 0.2)
  (bind _peer (CallFunction|RelayNetAuthorityfor _self))
  (bind _returnvalue (CallFunction|RelayVoiceBindSink _peer (Variables|Default|GetVoice_Chat) _self))
  (Variables|Default|SetVoiceSink _returnvalue)
  (bind _deviceid (CallFunction|RelayVoiceGetPreferredDevice))
  (bind _returnvalue_2 (CallFunction|RelayVoiceOpen _deviceid "NewEnumerator3" self))
  (Variables|Default|SetVoice _returnvalue_2))

(event EventTick
  (params (DeltaSeconds :type Float%20%28single-precision%29))
  (bind _relaycameraanchor (Variables|Default|GetRelayCameraAnchor))
  (bind (_value _valid) (CallFunction|RelayNetCameraLocation self))
  (bind (_value_2 _valid_2) (CallFunction|RelayNetCameraRotation self))
  (if (and _valid _valid_2)
    (Transformation|SetWorldLocation _relaycameraanchor _value false false)
    (Transformation|SetWorldRotation _relaycameraanchor _value_2 false false)))

(event Input|KeyboardEvents|B
  (params (Key :type Key%20Structure :default "None")))

(fn ConstructionScript
  (|CallParentFunction))